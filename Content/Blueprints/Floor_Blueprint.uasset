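; Floor actor that continuously rocks back and forth, tilting between positive and negative RotationAmount on its roll.
; Each Tick reads the actor's roll, flips the RoateLeft flag once it passes a limit, and otherwise adds a small fixed local rotation in the current direction.
; The step ignores delta time, so the rocking speed depends on frame rate.
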(event EventBeginPlay)

(event Collision|EventActorBeginOverlap
  (params (OtherActor :type Actor%20Object%20Reference)))

(event EventTick
  (params (DeltaSeconds :type Float%20%28single-precision%29))
  (bind _returnvalue (Transformation|GetActorRotation))
  (bind _rotationamount (Variables|Default|GetrotationAmount))
  (bind _roll (Math|Rotator|BreakRotator _returnvalue))
  (if (Variables|Default|GetroateLeft)
    (if (> _roll _rotationamount)
      (Variables|Default|SetroateLeft false)
      (else
        (Transformation|AddActorLocalRotation "0, 0,0.010000" false false)))
    (elif (< _roll (* _rotationamount -1.0))
      (Variables|Default|SetroateLeft true)
      (else
        (Transformation|AddActorLocalRotation "0, 0,-0.010000" false false)))))

(fn ConstructionScript)