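; Cannonball projectile actor that propels its Ball component along the actor's forward direction and removes itself after a short lifetime.
; BeginPlay scales the Ball to half size.
; Every Tick adds a mass-independent velocity-change impulse, so the push repeats each frame rather than firing once at launch.
; A Delay on the same Tick chain destroys the actor five seconds after the first tick.
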(event EventTick
  (params (DeltaSeconds :type Float%20%28single-precision%29))
  (Physics|AddImpulse (Variables|Default|GetBall) (* (Math|Vector|Normalize (Math|Vector|GetForwardVector (Transformation|GetActorRotation))) 2.5e+03) "None" true)
  (Utilities|FlowControl|Delay 5.0)
  (Actor|DestroyActor))

(event EventBeginPlay
  (Transformation|SetWorldScale3D (Variables|Default|GetBall) "0.500000,0.500000,0.500000"))

(fn ConstructionScript)