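; Spawner actor that places a set number of BP_Cannonball actors (despite the enemy naming) within its BoxCollider area at BeginPlay.
; Each spawn line-traces from high above random box points along the actor's down vector against WorldStatic, with debug drawing.
; It spawns slightly above the impact point without checking for a hit, using a random yaw of only 0–1 degree.
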(event EventBeginPlay
  (for _index (range 1 (Variables|Default|GetEnemySpawnCount))
    (CallFunction|SpawnEnemy)))

(fn ConstructionScript)

(fn SpawnEnemy
  (bind _boxcollider (Variables|Default|GetBoxCollider))
  (bind (_origin _boxextent) (Collision|GetComponentBounds _boxcollider))
  (bind _returnvalue (Math|Random|RandomPointinBoundingBox _origin _boxextent))
  (bind (_x _y _z) (Math|Vector|BreakVector _returnvalue))
  (bind _returnvalue_2 (+ _z 1e+04))
  (bind _returnvalue_3 (Math|Vector|MakeVector _x _y _returnvalue_2))
  ;[1 1 1] Spawn at LineTrace Impact Point
  (bind _outhit (Collision|LineTraceForObjects _returnvalue_3 (+ _returnvalue_3 (* (* (Transformation|GetActorUpVector) -1) 1.5e+04)) (Utilities|Array|MakeArray "ObjectTypeQuery1") false 0 "ForDuration"))
  (Game|SpawnActorfromClass "/Game/Blueprints/BP_Cannonball.BP_Cannonball_C" (Math|Transform|MakeTransform (+ (.ImpactPoint (Collision|BreakHitResult _outhit)) "0, 0,50.000000") (Math|Rotator|MakeRotator 0.0 0.0 (Math|Random|RandomFloat))) "Undefined" 0 0))