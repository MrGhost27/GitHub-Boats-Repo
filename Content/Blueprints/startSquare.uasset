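; Start square actor that counts down while all spawned players stand on it, then hides itself and starts enemy spawning.
; Tick compares overlapping and spawned player counts, showing a frame-based 500-tick countdown on Counter and resetting it when they differ.
; SpawnEnemies cycles through every BP_EnemySpawner until EnemiesToSpawn is reached, possibly overshooting because each pass finishes.
; Neither player count is updated in these graphs.
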(event EventBeginPlay
  (Rendering|Components|TextRender|SetText (Variables|Default|GetCounter) (Variables|Default|GetdefaultText)))

(event Collision|EventActorBeginOverlap
  (params (OtherActor :type Actor%20Object%20Reference)))

(event EventTick
  (params (DeltaSeconds :type Float%20%28single-precision%29))
  (bind _spawnedplayers (Variables|Default|GetspawnedPlayers))
  (if (and (== (Variables|Default|GetoverlappingPlayers) _spawnedplayers) (> _spawnedplayers 0.0))
    (bind _result (Math|Float|IncrementFloat (Variables|Default|GetTimer))
      (:%20%20
        (Rendering|Components|TextRender|SetText (Variables|Default|GetCounter) (Utilities|Text|ToText(Float) (- 5e+02 _result) "HalfToEven"))
        (if (> _result 5e+02)
          (Rendering|SetVisibility (Variables|Default|GetDefaultSceneRoot) false true)
          (CallFunction|SpawnEnemies))))
    (else
      (Variables|Default|SetTimer 0.0)
      (Rendering|Components|TextRender|SetText (Variables|Default|GetCounter) (Variables|Default|GetdefaultText)))))

(fn ConstructionScript)

(fn SpawnEnemies
  (bind _outactors (Actor|GetAllActorsOfClass "/Game/Blueprints/BP_EnemySpawner.BP_EnemySpawner_C"))
  (while (< (Variables|Default|GetenemiesSpawned) (Variables|Default|GetenemiesToSpawn))
    (for _array_element _outactors
      (Default|SpawnEnemy _array_element)
      (Math|Float|IncrementFloat (Variables|Default|GetenemiesSpawned)))))