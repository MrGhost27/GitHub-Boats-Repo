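; Cannonball store actor that lets the player pick up a cannonball while standing in its trigger box.
; Box overlap toggles player-zero input and the Press prompt's visibility, without checking which actor overlaps.
; Pressing Action inside the box, gated by PlayerHasBall, calls RetrieveCannonball, which shows the BPCPlayer reference's Cannonball and sets HasCannonball if it was not already set.
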(event OnComponentBeginOverlap(BoxTrigger)
  (params (OverlappedComponent :type Primitive%20Component%20Object%20Reference) (OtherActor :type Actor%20Object%20Reference) (OtherComp :type Primitive%20Component%20Object%20Reference) (OtherBodyIndex :type Integer) (bFromSweep :type Boolean) (SweepResult :type Hit%20Result%20Structure%20%28by%20ref%29))
  (Variables|Default|SetInBox true)
  (Input|EnableInput (Game|GetPlayerController 0))
  (Rendering|SetVisibility (Variables|Default|GetPress) (Variables|Default|GetInBox) false))

(event OnComponentEndOverlap(BoxTrigger)
  (params (OverlappedComponent :type Primitive%20Component%20Object%20Reference) (OtherActor :type Actor%20Object%20Reference) (OtherComp :type Primitive%20Component%20Object%20Reference) (OtherBodyIndex :type Integer))
  (Variables|Default|SetInBox false)
  (Input|DisableInput (Game|GetPlayerController 0))
  (Rendering|SetVisibility (Variables|Default|GetPress) (Variables|Default|GetInBox) false))

(event EventBeginPlay)

(event Collision|EventActorBeginOverlap
  (params (OtherActor :type Actor%20Object%20Reference)))

(event EventTick
  (params (DeltaSeconds :type Float%20%28single-precision%29)))

(event Input|ActionEvents|InputActionAction
  (params (Key :type Key%20Structure :default "None"))
  (:Pressed
    (if (Variables|Default|GetInBox)
      (if (not (Variables|Default|GetPlayerHasBall))
        (CallFunction|RetrieveCannonball)))))

(fn ConstructionScript)

(fn RetrieveCannonball
  (bind _bp_c__player (Variables|Default|GetBP_C++Player))
  (if (not (Variables|/Script/BlankBoats.PlayerCharacter|GethasCannonball _bp_c__player))
    (Rendering|SetVisibility (Variables|/Script/BlankBoats.PlayerCharacter|GetCannonball _bp_c__player) true true)
    (Variables|/Script/BlankBoats.PlayerCharacter|SethasCannonball _bp_c__player true)))