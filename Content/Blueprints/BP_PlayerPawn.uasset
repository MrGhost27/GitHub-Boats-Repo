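; BP_PlayerPawn is a player pawn with axis-driven movement, a dash and a timer UI widget shown on BeginPlay.
; Forward and right axes set scaled speeds, which Tick adds to the world location as X and Y offsets, without sweep or delta-time scaling.
; Dash bypasses that path by setting the FloatingPawnMovement velocity along the actor's forward vector, scaled by DashForce.
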(event EventBeginPlay
  (bind _returnvalue (UserInterface|CreateWidget "/Game/Blueprints/WBP_TimerUI.WBP_TimerUI_C"))
  (bind _output_get (Variables|Default|SetBP_PlayerHUD _returnvalue))
  (UserInterface|Viewport|AddtoViewport _output_get 0))

(event Collision|EventActorBeginOverlap
  (params (OtherActor :type Actor%20Object%20Reference)))

(event EventTick
  (params (DeltaSeconds :type Float%20%28single-precision%29))
  (Variables|Default|SetDeltaSeconds DeltaSeconds)
  (Transformation|SetActorLocation (+ (Math|Vector|MakeVector (Variables|Default|GetVerSpeed) (Variables|Default|GetHorSpeed) 0.0) (Transformation|GetActorLocation)) false false))

(event Input|ActionEvents|InputActionDash
  (params (Key :type Key%20Structure :default "None"))
  (:Pressed
    (Variables|/Script/Engine.MovementComponent|SetVelocity (Variables|Default|GetFloatingPawnMovement) (* (Math|Vector|Normalize (Math|Vector|GetForwardVector (Transformation|GetActorRotation))) (Variables|Default|GetDashForce)))))

(event Input|AxisEvents|InputAxisForwardMoveAxis
  (params (AxisValue :type Float%20%28single-precision%29))
  (Variables|Default|SetVerSpeed (* AxisValue (Variables|Default|GetSpeedMultiplier))))

(event Input|AxisEvents|InputAxisRightMoveAxis
  (params (AxisValue :type Float%20%28single-precision%29))
  (Variables|Default|SetHorSpeed (* AxisValue (Variables|Default|GetSpeedMultiplier))))

(fn ConstructionScript)