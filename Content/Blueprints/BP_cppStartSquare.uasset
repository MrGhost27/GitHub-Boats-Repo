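; BP_cppStartSquare is a start zone that counts overlapping player characters and resets the game through BP_GameMode.
; It registers itself with the game mode on BeginPlay, and calls ResetGame whenever UpdateTimer, defined outside these graphs, returns true on Tick.
; SpawnEnemies cycles through every BP_EnemySpawner until the target count is reached, checking only between full passes, so it can overshoot.
; OnEndGame is empty.
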(event Collision|EventActorEndOverlap
  (params (OtherActor :type Actor%20Object%20Reference))
  (Utilities|Casting|CastToBP_CPPPlayerCharacter OtherActor)
  (Math|Integer|DecrementInt (Variables|Default|GetoverlappingPlayers)))

(event Collision|EventActorBeginOverlap
  (params (OtherActor :type Actor%20Object%20Reference))
  (Utilities|Casting|CastToBP_CPPPlayerCharacter OtherActor)
  (Math|Integer|IncrementInt (Variables|Default|GetoverlappingPlayers)))

(event EventTick
  (params (DeltaSeconds :type Float%20%28single-precision%29))
  (bind _returnvalue (Class|CppStartSquare|UpdateTimer))
  (if _returnvalue
    (bind _asbp_game_mode (Utilities|Casting|CastToBP_GameMode (Game|GetGameMode)))
    (Default|ResetGame _asbp_game_mode)))

(event EventBeginPlay
  (bind _asbp_game_mode (Utilities|Casting|CastToBP_GameMode (Game|GetGameMode)))
  (Variables|/Game/Blueprints/BP_GameMode.BP_GameMode_C|SetStartSquare _asbp_game_mode self))

(fn ConstructionScript)

(fn SpawnEnemies
  (bind _outactors (Actor|GetAllActorsOfClass "/Game/Blueprints/BP_EnemySpawner.BP_EnemySpawner_C"))
  (while (< (Variables|Default|GetenemiesSpawned) (Variables|Default|GetenemiesToSpawn))
    (for _array_element _outactors
      (Default|SpawnEnemy _array_element)
      (Math|Integer|IncrementInt (Variables|Default|GetenemiesSpawned)))))

(fn OnEndGame)