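; AI controller for enemy guards that runs their behavior tree and exposes helpers for movement and attacking the player's home.
; On possess it caches the game mode, starts the EnemyGuard behavior tree and stores its blackboard.
; Helper functions write a move-to location into the blackboard and tell the game mode that the home takes damage.
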(event EventPossess
  (params (PossessedPawn :type Pawn%20Object%20Reference))
  (bind _asbp_game_mode (Utilities|Casting|CastToBP_GameMode (Game|GetGameMode)))
  (Variables|Default|SetGameModeRef _asbp_game_mode)
  (AI|RunBehaviorTree "/Game/Blueprints/AI/BT_EnemyGuard.BT_EnemyGuard")
  (bind _blackboardcomponent (Class|AIController|UseBlackboard "/Game/Blueprints/AI/BB_EnemyGuard.BB_EnemyGuard"))
  (Variables|Default|SetBlackboard%20Ref _blackboardcomponent))

(fn ConstructionScript)

(fn SetMovetoLocation
  (params (DesiredLocation :type Vector))
  (AI|Components|Blackboard|SetValueasVector (Variables|Default|GetBlackboard%20Ref) (Variables|Default|GetMoveToLocationKey) DesiredLocation))

(fn DamagePlayerHome
  (Default|HomeTakesDamage (Variables|Default|GetGameModeRef)))