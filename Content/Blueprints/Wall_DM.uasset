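; Wall_DM is a destructible wall actor that slides along the world Y axis and reacts to cannonball hits.
; Each tick it grows an offset from its starting location by a fixed, frame-rate-dependent step, with MoveLeft choosing the direction; nothing here toggles that flag.
; When a BP_CannonballProjectile hits the Destructible component, it applies point damage to the hit result's actor, passing the impact point as the direction.
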(event OnComponentHit(Destructible)
  (params (HitComponent :type Primitive%20Component%20Object%20Reference) (OtherActor :type Actor%20Object%20Reference) (OtherComp :type Primitive%20Component%20Object%20Reference) (NormalImpulse :type Vector :default "0, 0, 0") (Hit :type Hit%20Result%20Structure%20%28by%20ref%29))
  (bind (_bblockinghit _binitialoverlap _time _distance _location _impactpoint _normal _impactnormal _physmat _hitactor) (Collision|BreakHitResult Hit))
  (bind _asbp_cannonball_projectile (Utilities|Casting|CastToBP_CannonballProjectile OtherActor))
  (Game|Damage|ApplyPointDamage _hitactor 1e+02 _impactpoint Hit 0 _asbp_cannonball_projectile "/Script/Engine.DamageType"))

(event EventBeginPlay
  (Variables|Default|SetinitialPos (Transformation|GetActorLocation)))

(event Collision|EventActorBeginOverlap
  (params (OtherActor :type Actor%20Object%20Reference)))

(event EventTick
  (params (DeltaSeconds :type Float%20%28single-precision%29))
  (bind _initialpos (Variables|Default|GetinitialPos))
  (if (Variables|Default|GetmoveLeft)
    (bind _output_get (Variables|Default|SetoffsetPos (+ (Variables|Default|GetoffsetPos) "0,1.000000, 0")))
    (Transformation|SetActorLocation (+ _output_get _initialpos) false false)
    (else
      (bind _output_get_2 (Variables|Default|SetoffsetPos (+ (Variables|Default|GetoffsetPos) "0,-1.000000, 0")))
      (Transformation|SetActorLocation (+ _initialpos _output_get_2) false false))))

(fn ConstructionScript)