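; BP_Cannon is an interactable cannon that the player can fire when it is loaded with a ball.
; A Box trigger sets InBox, enables or disables the first player controller's input on the cannon, and shows or hides the Press prompt to match.
; Pressing Interact while HasBall is true spawns a BP_Cannonball at the CannonballSpawn transform through FireCannon, then clears HasBall; nothing in these graphs sets it again.
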(event OnComponentBeginOverlap(Box)
  (params (OverlappedComponent :type Primitive%20Component%20Object%20Reference) (OtherActor :type Actor%20Object%20Reference) (OtherComp :type Primitive%20Component%20Object%20Reference) (OtherBodyIndex :type Integer) (bFromSweep :type Boolean) (SweepResult :type Hit%20Result%20Structure%20%28by%20ref%29))
  (Variables|Default|SetInBox true)
  (Input|EnableInput (Game|GetPlayerController 0))
  (Rendering|SetVisibility (Variables|Default|GetPress) (Variables|Default|GetInBox) false))

(event OnComponentEndOverlap(Box)
  (params (OverlappedComponent :type Primitive%20Component%20Object%20Reference) (OtherActor :type Actor%20Object%20Reference) (OtherComp :type Primitive%20Component%20Object%20Reference) (OtherBodyIndex :type Integer))
  (Variables|Default|SetInBox false)
  (Input|DisableInput (Game|GetPlayerController 0))
  (Rendering|SetVisibility (Variables|Default|GetPress) (Variables|Default|GetInBox) false))

(event EventBeginPlay)

(event Collision|EventActorBeginOverlap
  (params (OtherActor :type Actor%20Object%20Reference)))

(event EventTick
  (params (DeltaSeconds :type Float%20%28single-precision%29)))

(event Input|ActionEvents|InputActionInteract
  (params (Key :type Key%20Structure :default "None"))
  (:Pressed
    (if (Variables|Default|GetHasBall)
      (CallFunction|FireCannon (Transformation|GetWorldTransform (Variables|Default|GetCannonballSpawn)))
      (Variables|Default|SetHasBall false))))

(fn ConstructionScript)

(fn FireCannon
  (params (SpawnLocation :type Transform))
  (Game|SpawnActorfromClass "/Game/Blueprints/BP_Cannonball.BP_Cannonball_C" SpawnLocation "AlwaysSpawn" 0 0))