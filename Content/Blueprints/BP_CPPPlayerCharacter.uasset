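; Player character Blueprint that picks up, carries, releases and throws physics objects, with special tracking for cannonballs.
; A forward line trace grabs objects under the carry weight limit with a runtime-added PhysicsHandle, steered each Tick to the HoldDistnace component.
; Yeet releases the object with a forward velocity impulse and clears the cannonball's HeldByPlayer flag.
; Capsule overlap with the CB actor switches the character mesh to physics simulation.
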(event OnComponentBeginOverlap(CapsuleComponent)
  (params (OverlappedComponent :type Primitive%20Component%20Object%20Reference) (OtherActor :type Actor%20Object%20Reference) (OtherComp :type Primitive%20Component%20Object%20Reference) (OtherBodyIndex :type Integer) (bFromSweep :type Boolean) (SweepResult :type Hit%20Result%20Structure%20%28by%20ref%29))
  (if (== OtherActor (Variables|Default|GetCB))
    (Physics|SetSimulatePhysics (Variables|Character|GetMesh) true)))

(event EventTick
  (params (DeltaSeconds :type Float%20%28single-precision%29))
  (CallFunction|SetPhysicsHandleLocation))

(event Input|ActionEvents|InputActionPickupObject
  (params (Key :type Key%20Structure :default "None"))
  (:Pressed
    (CallFunction|PickUpObject))
  (:Released
    (CallFunction|ReleaseObject)))

(event Input|ActionEvents|InputActionYeet
  (params (Key :type Key%20Structure :default "None"))
  (:Pressed
    (CallFunction|Yeet))
  (:Released
    (Variables|Default|SetisHeld false)))

(event Input|KeyboardEvents|G
  (params (Key :type Key%20Structure :default "None")))

(fn ConstructionScript)

(fn PickUpObject
  (bind _mesh (Variables|Character|GetMesh))
  (bind _returnvalue (Transformation|GetWorldLocation _mesh))
  (Variables|Default|SetPhysicsHandleActive true)
  (bind (_outhit _returnvalue_2) (Collision|LineTraceForObjects _returnvalue (+ _returnvalue (* (Math|Vector|GetForwardVector _mesh) (Variables|Default|GetPickUpDistance))) (Variables|Default|GetPhysicsObjectType) false 0 "ForDuration"))
  (Variables|Default|SetObjectLocation (Math|Vector|VectorLength (- (Transformation|GetActorLocation) (.Location (Collision|BreakHitResult _outhit)))))
  (Variables|Default|SetObjectRotation (Transformation|GetActorRotation))
  (if _returnvalue_2
    (if (< (Physics|GetMass (.HitComponent (Collision|BreakHitResult _outhit))) (Variables|Default|GetCarryWeightLimit)) ; Check weight of object is less than carry strength
      (bind _returnvalue_3 (AddComponent|AddPhysicsHandleComponent (Transformation|GetActorTransform)))
      (Variables|Default|SetPhysicsHandle _returnvalue_3)
      (Variables|Default|SetPhysicsObject (.HitComponent (Collision|BreakHitResult _outhit)))
      (Physics|Components|PhysicsHandle|GrabComponentatLocationwithRotation (Variables|Default|GetPhysicsHandle) (.HitComponent (Collision|BreakHitResult _outhit)) (.HitBoneName (Collision|BreakHitResult _outhit)) (- (.Location (Collision|BreakHitResult _outhit)) "0,-10.000000,0.000000") "0, 0, 0")
      (Collision|SetCollisionResponsetoChannel (Variables|Character|GetMesh) "ECC_Pawn" "ECR_Ignore")
      (Variables|Default|SethasCannonball true)
      (bind _asbp_cannonball (Utilities|Casting|CastToBP_Cannonball (.HitActor (Collision|BreakHitResult _outhit))))
      (Variables|/Game/Blueprints/BP_Cannonball.BP_Cannonball_C|SetHeldByPlayer _asbp_cannonball true))))

(fn ReleaseObject
  (bind _physicsobject (Variables|Default|GetPhysicsObject))
  (Variables|Default|SetPhysicsHandleActive false)
  (Physics|Components|PhysicsHandle|ReleaseComponent (Variables|Default|GetPhysicsHandle))
  (if (Variables|Default|GetisHeld)
    (Class|PrimitiveComponent|WakeRigidBody _physicsobject "None"))
  (Collision|SetCollisionResponsetoChannel _physicsobject "ECC_Pawn" "ECR_Ignore")
  (Variables|Default|SethasCannonball false)
  (bind _asbp_cannonball (Utilities|Casting|CastToBP_Cannonball (Components|GetOwner _physicsobject)))
  (Variables|/Game/Blueprints/BP_Cannonball.BP_Cannonball_C|SetHeldByPlayer _asbp_cannonball true))

(fn Yeet
  (bind _physicsobject (Variables|Default|GetPhysicsObject))
  (bind _returnvalue (Components|GetOwner _physicsobject))
  (Variables|Default|SetisHeld true)
  (if (Variables|Default|GetPhysicsHandleActive)
    (Variables|Default|SetPhysicsHandleActive false)
    (Physics|Components|PhysicsHandle|ReleaseComponent (Variables|Default|GetPhysicsHandle))
    (if (Variables|Default|GetisHeld)
      (Class|PrimitiveComponent|WakeRigidBody _physicsobject "None"))
    (Collision|SetCollisionResponsetoChannel _physicsobject "ECC_Pawn" "ECR_Ignore")
    (Variables|Default|SethasCannonball false)
    (if (== (Utilities|GetClass _returnvalue) "/Game/Blueprints/BP_Cannonball.BP_Cannonball_C")
      (bind _asbp_cannonball (Utilities|Casting|CastToBP_Cannonball _returnvalue))
      (Variables|/Game/Blueprints/BP_Cannonball.BP_Cannonball_C|SetHeldByPlayer _asbp_cannonball false))
    (Physics|AddImpulse _physicsobject (* (Math|Vector|GetForwardVector (Variables|Character|GetMesh)) 1e+03) "None" true)))

(fn SetPhysicsHandleLocation
  (if (Variables|Default|GetPhysicsHandleActive)
    (Variables|Default|SetHandleLocation (+ (+ (* (Math|Vector|GetForwardVector (Pawn|GetControlRotation :!class /Script/Engine.Pawn)) (Variables|Default|GetObjectLocation)) (Transformation|GetActorLocation)) "0,0.000000,-20.000000"))
    (Class|PhysicsHandleComponent|SetTargetLocationandRotation (Variables|Default|GetPhysicsHandle) (Transformation|GetWorldLocation (Variables|Default|GetHoldDistnace)) (Transformation|GetActorRotation))))