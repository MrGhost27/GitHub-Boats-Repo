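; Player character Blueprint that handles axis-driven movement and a dash.
; Forward and right inputs, scaled by a speed multiplier, set two speeds that Tick adds to the actor's location along world X and Y.
; This offset bypasses the movement component, with no sweep and no delta-time scaling.
; Pressing Dash instead overwrites the CharacterMovement velocity with the actor's forward direction times the dash force.
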(event EventTick
  (params (DeltaSeconds :type Float%20%28single-precision%29))
  (Variables|Default|SetDeltaSeconds DeltaSeconds)
  (Transformation|SetActorLocation (+ (Transformation|GetActorLocation) (Math|Vector|MakeVector (Variables|Default|GetVerSpeed) (Variables|Default|GetHorSpeed) 0.0)) false false))

(event Input|ActionEvents|InputActionDash
  (params (Key :type Key%20Structure :default "None"))
  (:Pressed
    (Variables|/Script/Engine.MovementComponent|SetVelocity (Variables|Character|GetCharacterMovement) (* (Math|Vector|Normalize (Math|Vector|GetForwardVector (Transformation|GetActorRotation))) (Variables|Default|GetDashForce)))))

(event Input|AxisEvents|InputAxisForwardMoveAxis
  (params (AxisValue :type Float%20%28single-precision%29))
  (Variables|Default|SetVerSpeed (* AxisValue (Variables|Default|GetSpeedMultiplier))))

(event Input|AxisEvents|InputAxisRightMoveAxis
  (params (AxisValue :type Float%20%28single-precision%29))
  (Variables|Default|SetHorSpeed (* AxisValue (Variables|Default|GetSpeedMultiplier))))

(fn ConstructionScript)